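; BP_TriggerWall is a trigger box that switches the player's camera mode while something overlaps it.
; Begin overlap sends the configured mode, plus an optional TopDownCamera, to player character 0 via an interface message, without checking which actor overlapped.
; End overlap resets the mode to the enum's first entry.
; The construction script clears TopDownCamera unless top-down mode is selected; its own Get/SetCameraMode functions are stubs.
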(event `self.Box.OnComponentBeginOverlap`
  (params (OverlappedComponent :type "PrimitiveComponent Object Reference") (OtherActor :type "Actor Object Reference") (OtherComp :type "PrimitiveComponent Object Reference") (OtherBodyIndex :type Integer) (bFromSweep :type Boolean) (SweepResult :type "HitResult Structure (by ref)"))
  (`self.TopDownCamera`
    (:`then`
      (message `/Game/SPINE/Blueprints/BPI_PlayerCharacter.SetCameraMode` (`GameplayStatics.GetPlayerCharacter` 0) (`self.CameraModeToSwitch`) (`self.TopDownCamera`)))
    (:`else`
      (message `/Game/SPINE/Blueprints/BPI_PlayerCharacter.SetCameraMode` (`GameplayStatics.GetPlayerCharacter` 0) (`self.CameraModeToSwitch`) null))))

(event `self.Box.OnComponentEndOverlap`
  (params (OverlappedComponent :type "PrimitiveComponent Object Reference") (OtherActor :type "Actor Object Reference") (OtherComp :type "PrimitiveComponent Object Reference") (OtherBodyIndex :type Integer))
  (message `/Game/SPINE/Blueprints/BPI_PlayerCharacter.SetCameraMode` (`GameplayStatics.GetPlayerCharacter` 0) "NewEnumerator0" null))

(fn `GetCameraMode`
  (returns (CurrentCameraMode :type "/Game/SPINE/Blueprints/ECameraMode Enum"))
  (return "NewEnumerator0"))

(fn `SetCameraMode`
  (params (CameraModeToSet :type "/Game/SPINE/Blueprints/ECameraMode Enum" :default "NewEnumerator0") (TopDownCamera :type "/Game/SPINE/Blueprints/BP_TopDownCameraPoint Object Reference")))

(fn `UserConstructionScript`
  ;[0 0 0] Does not allow to set camera, if CameraModeToSwitch does not equal TopDownCamera
  (if (`|EnumInequality` (`self.CameraModeToSwitch`) "NewEnumerator1")
    (set `self.TopDownCamera` null)))